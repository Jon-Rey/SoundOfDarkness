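; VR tuner pickup that a motion controller can grab and drop, sounding and triggering a glow-outline effect when its audio box overlaps something.
; Each strike plays the first idle of five audio components, fading it over the sound's length, so rings can overlap.
; A timeline simultaneously animates a post-process dynamic material, created in Init, through Radius and Thing parameters.
; A DoOnce blocks retriggers until an end overlap leaves one overlapping actor.
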(event OnComponentBeginOverlap(BoxOverlapAudio)
  (params (OverlappedComponent :type Primitive%20Component%20Object%20Reference) (OtherActor :type Actor%20Object%20Reference) (OtherComp :type Primitive%20Component%20Object%20Reference) (OtherBodyIndex :type Integer) (bFromSweep :type Boolean) (SweepResult :type Hit%20Result%20Structure%20%28by%20ref%29))
  (bind _audio1 (Variables|Default|GetAudio1))
  (bind _audio (Variables|Default|GetAudio))
  (bind _audio2 (Variables|Default|GetAudio2))
  (bind _audio3 (Variables|Default|GetAudio3))
  (bind _audio4 (Variables|Default|GetAudio4))
  (bind _audio_2 (Variables|Default|GetAudio))
  (bind _material (Variables|Default|GetMaterial))
  (Utilities|FlowControl|DoOnce false
    (:Completed
      (Utilities|FlowControl|Sequence
        (:then_0
          (if (Audio|Components|Audio|IsPlaying _audio_2)
            (if (Audio|Components|Audio|IsPlaying _audio2)
              (if (Audio|Components|Audio|IsPlaying _audio1)
                (if (Audio|Components|Audio|IsPlaying _audio3)
                  (if (Audio|Components|Audio|IsPlaying _audio4)
                    (Audio|Components|Audio|Play _audio 0.1)
                    (Audio|Components|Audio|AdjustVolume _audio (Variables|/Script/Engine.SoundBase|GetDuration (Variables|/Script/Engine.AudioComponent|GetSound _audio)) 0.0 :!class /Script/Engine.AudioComponent)
                    (else
                      (Audio|Components|Audio|Play _audio4 0.1)
                      (Audio|Components|Audio|AdjustVolume _audio4 (Variables|/Script/Engine.SoundBase|GetDuration (Variables|/Script/Engine.AudioComponent|GetSound _audio4)) 0.0 :!class /Script/Engine.AudioComponent)))
                  (else
                    (Audio|Components|Audio|Play _audio3 0.1)
                    (Audio|Components|Audio|AdjustVolume _audio3 (Variables|/Script/Engine.SoundBase|GetDuration (Variables|/Script/Engine.AudioComponent|GetSound _audio3)) 0.0 :!class /Script/Engine.AudioComponent)))
                (else
                  (Audio|Components|Audio|Play _audio1 0.1)
                  (Audio|Components|Audio|AdjustVolume _audio1 (Variables|/Script/Engine.SoundBase|GetDuration (Variables|/Script/Engine.AudioComponent|GetSound _audio1)) 0.0 :!class /Script/Engine.AudioComponent)))
              (else
                (Audio|Components|Audio|Play _audio2 0.1)
                (Audio|Components|Audio|AdjustVolume _audio2 (Variables|/Script/Engine.SoundBase|GetDuration (Variables|/Script/Engine.AudioComponent|GetSound _audio2)) 0.0 :!class /Script/Engine.AudioComponent)))
            (else
              (Audio|Components|Audio|Play _audio_2 0.1)
              (Audio|Components|Audio|AdjustVolume _audio_2 (Variables|/Script/Engine.SoundBase|GetDuration (Variables|/Script/Engine.AudioComponent|GetSound _audio_2)) 0.0 :!class /Script/Engine.AudioComponent))))
        (:then_1
          (bind (_direction _r _t) (Timeline|DoTheThing PlayFromStart)
            (:Update
              (Rendering|Material|SetScalarParameterValue _material "Radius" _r :!class /Script/Engine.MaterialInstanceDynamic)
              (Rendering|Material|SetScalarParameterValue _material "Thing" _t :!class /Script/Engine.MaterialInstanceDynamic))))))))

(event OnComponentEndOverlap(BoxOverlapAudio)
  (params (OverlappedComponent :type Primitive%20Component%20Object%20Reference) (OtherActor :type Actor%20Object%20Reference) (OtherComp :type Primitive%20Component%20Object%20Reference) (OtherBodyIndex :type Integer))
  (bind _audio1 (Variables|Default|GetAudio1))
  (bind _audio (Variables|Default|GetAudio))
  (bind _audio2 (Variables|Default|GetAudio2))
  (bind _audio3 (Variables|Default|GetAudio3))
  (bind _audio4 (Variables|Default|GetAudio4))
  (bind _audio_2 (Variables|Default|GetAudio))
  (bind _material (Variables|Default|GetMaterial))
  (if (== (Utilities|Array|Length (Collision|GetOverlappingActors 0 :!class /Script/Engine.Actor)) 1)
    (Utilities|FlowControl|DoOnce false) ; enters at Reset
  ))

(event Custom|Init
  (bind _returnvalue (Rendering|Material|CreateDynamicMaterialInstance "/Game/_SoundOfDarkness/Materials/GlowOutlineMat_Inst.GlowOutlineMat_Inst" "None" :!class /Script/Engine.KismetMaterialLibrary))
  (bind _output_get (Variables|Default|SetMaterial _returnvalue))
  (Variables|/Script/Engine.PostProcessVolume|SetSettings (Variables|Default|GetPostProcessVol) (Utilities|Struct|MakePostProcessSettings (Utilities|Struct|MakeWeightedBlendables (Utilities|Array|MakeArray (Utilities|Struct|MakeWeightedBlendable 1.0 _output_get))))))

(event EventBeginPlay
  (Audio|Components|Audio|Stop (Variables|Default|GetAudio))
  (Audio|Components|Audio|Stop (Variables|Default|GetAudio1))
  (Audio|Components|Audio|Stop (Variables|Default|GetAudio2))
  (Audio|Components|Audio|Stop (Variables|Default|GetAudio3))
  (Audio|Components|Audio|Stop (Variables|Default|GetAudio4)))

(event Collision|EventActorBeginOverlap
  (params (OtherActor :type Actor%20Object%20Reference)))

(event EventTick
  (params (DeltaSeconds :type Float%20%28single-precision%29)))

(event EventPickup
  (params (AttachTo :type Scene%20Component%20Object%20Reference))
  (Physics|SetSimulatePhysics (Variables|Debug|GetStaticMeshComponent) false)
  (Transformation|AttachComponentToComponent (VehicleSound|GetRootComponent) AttachTo "None" "SnapToTarget" "SnapToTarget" "KeepWorld" false)
  (Transformation|SetRelativeLocationAndRotation (Variables|Debug|GetStaticMeshComponent) "-5.180000,-0.501000,-1.850000" "-28.131001, 0, 0" false false))

(event EventDrop
  (Utilities|FlowControl|Sequence
    (:then_0
      (Physics|SetSimulatePhysics (Variables|Debug|GetStaticMeshComponent) true)
      (Transformation|DetachFromActor "KeepWorld" "KeepWorld" "KeepWorld"))))

(fn ConstructionScript)