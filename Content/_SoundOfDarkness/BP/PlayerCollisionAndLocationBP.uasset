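; VR player collision proxy that handles thumbstick locomotion and room-scale head movement, then positions the player pawn from the result.
; Each tick, left-stick input moves Pos along the headset's flattened axes, with strafing at half speed.
; Two swept moves test stick and head motion separately, ignoring BP_MotionController hits; blocked stick motion reverts, while blocked head motion shifts Pos back.
; PlayerPawn follows, offset by headset position and capsule half-height.
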(event EventBeginPlay
  (Variables|Default|SetPos (Transformation|GetActorLocation)))

(event Collision|EventActorBeginOverlap
  (params (OtherActor :type Actor%20Object%20Reference)))

(event EventTick
  (params (DeltaSeconds :type Float%20%28single-precision%29))
  (bind _deviceposition (Class|OculusFunctionLibrary|GetPose false true "0, 0, 0"))
  (bind _devicerotation (Class|OculusFunctionLibrary|GetPose false true "0, 0, 0"))
  (bind _deviceposition_2 (Class|OculusFunctionLibrary|GetPose false true "100.000000,100.000000, 0"))
  (bind _returnvalue (Transformation|GetActorLocation))
  (bind _returnvalue_2 (Input|AxisValues|GetMotionControllerThumbLeft_X))
  (bind _returnvalue_3 (Input|AxisValues|GetMotionControllerThumbLeft_Y))
  (bind _speed (Variables|Default|GetSpeed))
  (bind _speed_2 (Variables|Default|GetSpeed))
  (bind _returnvalue_4 (- _returnvalue _deviceposition))
  (bind (_x _y) (Math|Rotator|BreakRotIntoAxes _devicerotation))
  (bind _returnvalue_5 (* DeltaSeconds _returnvalue_2 _speed 0.5))
  (bind _returnvalue_6 (* DeltaSeconds _returnvalue_3 _speed_2))
  (bind _returnvalue_7 (Math|Vector|ProjectVectorontoPlane _x "0, 0,1.000000"))
  (bind _returnvalue_8 (Math|Vector|ProjectVectorontoPlane _y "0, 0,1.000000"))
  (bind _returnvalue_9 (Math|Vector2D|Normalize2D (Math|Vector2D|MakeVector2D (.x _returnvalue_7) (.y _returnvalue_7))))
  (bind _returnvalue_10 (Math|Vector2D|Normalize2D (Math|Vector2D|MakeVector2D (.x _returnvalue_8) (.y _returnvalue_8))))
  (bind _returnvalue_11 (* _returnvalue_9 _returnvalue_6))
  (bind _returnvalue_12 (* _returnvalue_10 _returnvalue_5))
  (Variables|Default|SetPos (Math|Vector|MakeVector (+ (.x _returnvalue_11) (.x (Variables|Default|GetPos))) (+ (.y _returnvalue_11) (.y (Variables|Default|GetPos))) (.z (Variables|Default|GetPos))))
  (Variables|Default|SetPos (Math|Vector|MakeVector (+ (.x _returnvalue_12) (.x (Variables|Default|GetPos))) (+ (.y _returnvalue_12) (.y (Variables|Default|GetPos))) (.z (Variables|Default|GetPos))))
  (bind _sweephitresult (Transformation|SetActorLocation (+ (Variables|Default|GetPos) (Variables|Default|GetHeadPos)) true false))
  (if (.bBlockingHit (Collision|BreakHitResult _sweephitresult))
    (Utilities|Casting|CastToBP_MotionController (.HitActor (Collision|BreakHitResult _sweephitresult))
      (:then
        _)
      (:CastFailed
        (Variables|Default|SetPos (Variables|Default|GetLastPos)))))
  (Variables|Default|SetHeadPos (Math|Vector|MakeVector (.x _deviceposition_2) (.y _deviceposition_2) 0.0))
  (Variables|Default|SetLastPos (Variables|Default|GetPos))
  (bind _sweephitresult_2 (Transformation|SetActorLocation (+ (Variables|Default|GetPos) (Variables|Default|GetHeadPos)) true false))
  (if (.bBlockingHit (Collision|BreakHitResult _sweephitresult_2))
    (Utilities|Casting|CastToBP_MotionController (.HitActor (Collision|BreakHitResult _sweephitresult_2))
      (:then
        _)
      (:CastFailed
        (bind _output_get (Variables|Default|SetPos (- (Variables|Default|GetPos) (- (Variables|Default|GetHeadPos) (Variables|Default|GetLastHeadPos)))))
        (bind _output_get_2 (Variables|Default|SetHeadPos (Variables|Default|GetLastHeadPos)))
        (Transformation|SetActorLocation (+ _output_get _output_get_2) true false))))
  (Transformation|SetActorLocation (Variables|Default|GetPlayerPawn) (Math|Vector|MakeVector (.x _returnvalue_4) (.y _returnvalue_4) (- (.z (Transformation|GetActorLocation)) (Variables|/Script/Engine.CapsuleComponent|GetCapsuleHalfHeight (Variables|Default|GetCapsule)))) false false)
  (Variables|Default|SetLastHeadPos (Variables|Default|GetHeadPos)))

(fn ConstructionScript)